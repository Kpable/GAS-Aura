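; Electrocute lightning ability for Aura that caches mouse target and owner data, hides the cursor and turns the avatar toward the hit.
; An electrocute montage's gameplay event starts the shock loop and disables movement.
; The same Sequence immediately clears the loop, restores walking and ends the ability, without waiting for input release.
; The release handler sets the cursor hidden again, despite its restore label.
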(event Ability|EventActivateAbility
  (CallFunction|EnforceImplementsCombatInterface)
  ;[0.15 0.15 0.15 0.5] Store Mouse Data Variables
  (bind _datahandle (|TargetDataUnderMouse)
    (:then
      (Class|AuraBeamSpell|StoreMouseDataInfo (Ability|TargetData|GetHitResultfromTargetData _datahandle))
      (Class|AuraBeamSpell|StoreOwnerVariables)
      (Utilities|FlowControl|Sequence
        (:then_0
          ;[0.15 0.15 0.15 0.5] Hide Mouse Cursor
          (Variables|/Script/Engine.PlayerController|SetbShowMouseCursor (Variables|Default|GetOwnerPlayerController) false))
        (:then_1
          ;[0.15 0.15 0.15 0.5] Update Facing Target and Play Montage
          (Class|CombatInterface|UpdateFacingTarget(Message) (Ability|GetAvatarActorfromActorInfo) (Variables|Default|GetMouseHitLocation))
          (|PlayMontageandWaitProxy "None" (Variables|Beam|GetMontage_Electrocute) 1.0 "None" true 1.0 0.0 false
            (:then
              (Ability|Tasks|WaitGameplayEvent "(TagName=\"Event.Montage.Electrocute\")" 0 true
                (:EventReceived
                  ;[0.15 0.15 0.15 0.5] Enter Shock Loop
                  (Class|CombatInterface|SetinShockLoop(Message) (Ability|GetAvatarActorfromActorInfo) true)
                  ;[0.15 0.15 0.15 0.5] Disable Player Movement
                  (Pawn|Components|CharacterMovement|DisableMovement (Variables|/Script/Engine.Character|GetCharacterMovement (Variables|Default|GetOwnerCharacter))))))))
        (:then_3
          ;[0.15 0.15 0.15 0.5] Restore Mouse Cursor
          (Ability|Tasks|WaitInputRelease false
            (:OnRelease
              (Variables|/Script/Engine.PlayerController|SetbShowMouseCursor (Variables|Default|GetOwnerPlayerController) false))))
        (:then_4
          ;[0.15 0.15 0.15 0.5] Exit Shock Loop
          (Class|CombatInterface|SetinShockLoop(Message) (Ability|GetAvatarActorfromActorInfo) false)
          ;[0.15 0.15 0.15 0.5] Enable Player Movement
          (Pawn|Components|CharacterMovement|SetMovementMode (Variables|/Script/Engine.Character|GetCharacterMovement (Variables|Default|GetOwnerCharacter)) "MOVE_Walking" 0))
        (:then_5
          ;[0.15 0.15 0.15 0.5] End Ability
          (Ability|EndAbility))))))

(fn EnforceImplementsCombatInterface
  (if (not (Utilities|DoesObjectImplementInterface (Ability|GetAvatarActorfromActorInfo) "/Script/Aura.CombatInterface"))
    (Ability|EndAbility)))