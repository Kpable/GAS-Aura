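; GA_FireBolt is the Fire Bolt gameplay ability, which launches a projectile at the location under the mouse.
; On activation it gets target data under the mouse and turns the avatar to face the hit point through CombatInterface.
; It plays the cast montage and waits for the Event.Montage.FireBolt gameplay event, spawning the projectile toward that point when the event arrives.
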(event Ability|EventActivateAbility
  (bind _datahandle (|TargetDataUnderMouse)
    (:then
      (Variables|Default|SetProjectileHitTargetLocation (.Location (Collision|BreakHitResult (Ability|TargetData|GetHitResultfromTargetData _datahandle))))
      (bind _ascombat_interface (Utilities|Casting|CastToCombatInterface (Ability|GetAvatarActorfromActorInfo)))
      (Class|CombatInterface|UpdateFacingTarget _ascombat_interface (Variables|Default|GetProjectileHitTargetLocation))
      (|PlayMontageandWaitProxy "None" "/Game/Assets/Characters/Aura/Animations/Abilities/AM_Cast_FireBolt.AM_Cast_FireBolt" 1.0 "None" true 1.0 0.0 false
        (:then
          (Ability|Tasks|WaitGameplayEvent "(TagName=\"Event.Montage.FireBolt\")" 0
            (:EventReceived
              (Class|AuraProjectileSpell|SpawnProjectile (Variables|Default|GetProjectileHitTargetLocation)))))))))

(event Ability|EventOnEndAbility
  (params (bWasCancelled :type Boolean)))