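; BP_FlamePillar is a flame pillar actor whose point light flickers like fire.
; On BeginPlay it randomly plays one of two intensity timelines, then picks again each time one finishes, looping endlessly.
; Each timeline update sets the PointLight intensity to the curve value multiplied by BaseIntensity, so the flicker varies without a fixed repeating pattern.
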(event Custom|Choose%20Intensity
  (if (Math|Random|RandomBool)
    (CallFunction|ChooseFlameIntensity1)
    (else
      (CallFunction|ChooseFlameIntensity2))))

(event Custom|Choose%20Flame%20Intensity%201
  (bind _intensity (Timeline|Flame%20Intensity%201 PlayFromStart)
    (:Update
      (CallFunction|SetLightIntensity _intensity))
    (:Finished
      (CallFunction|ChooseIntensity))))

(event Custom|Choose%20Flame%20Intensity%202
  (bind _intensity (Timeline|Flame%20Intensity%202 PlayFromStart)
    (:Update
      (CallFunction|SetLightIntensity _intensity))
    (:Finished
      (CallFunction|ChooseIntensity))))

(event EventBeginPlay
  (CallFunction|ChooseIntensity))

(fn ConstructionScript)

(fn SetLightIntensity
  (params (Intensity :type Float%20%28double-precision%29))
  (Rendering|Components|Light|SetIntensity (Variables|Default|GetPointLight) (* Intensity (Variables|Default|GetBaseIntensity))))